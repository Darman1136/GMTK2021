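; Ability component from a 2021 game jam test bed that dashes the owning character along the camera's view direction, tilted upward.
; Using the ability applies a mass-independent velocity-change impulse to the character's physics actor and records the real-time timestamp.
; The readiness check combines the parent's check with a millisecond cooldown since the last dash, so game pause or time dilation does not affect it.
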(event `self.ReceiveTick`
  (params (DeltaSeconds :type "Float (single-precision)"))
  (`parent.ReceiveTick` DeltaSeconds))

(fn `InternalUseAbility`
  (returns (Success :type Boolean))
  (bind _castedcharacter (`self.CastedCharacter`))
  (bind _camera (`/Game/Maps/TestBeds/Mechanics/GameJam2021/BP_Slime_Character.Camera` _castedcharacter))
  (set `self.LastDash` (`KismetMathLibrary.GetTotalMilliseconds` (`KismetMathLibrary.FromSeconds` (`GameplayStatics.GetRealTimeSeconds`))))
  (`PrimitiveComponent.AddImpulse` (`/Game/Maps/TestBeds/Mechanics/GameJam2021/BP_Slime_Character.GetPhysicsActor` _castedcharacter) (* (`KismetMathLibrary.RotateAngleAxis` (`SceneComponent.GetForwardVector` _camera) -20.0 (`SceneComponent.GetRightVector` _camera)) 1000.0) "None" true)
  (return true))

(fn `IsReady`
  (returns (Ready :type Boolean))
  (return (and (`parent.IsReady`) (> (- (`KismetMathLibrary.GetTotalMilliseconds` (`KismetMathLibrary.FromSeconds` (`GameplayStatics.GetRealTimeSeconds`))) (`self.LastDash`)) (`self.DashDelayMs`)))))