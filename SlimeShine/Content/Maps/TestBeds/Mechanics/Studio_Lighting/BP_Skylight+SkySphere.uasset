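; Combined sky environment actor with a sky sphere, skylight, directional light and visible sun, which also handles hyperspace jump transitions.
; Construction script applies cubemap, color and sun settings through dynamic materials and recaptures the skylight, or hides everything when inactive.
; Tick optionally rotates sky and sun together, recapturing every frame.
; SwitchHyperspaceStage uses stage flags and timed delays to hide the space environment on tunnel entry and restore it on exit.
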(event `self.ReceiveBeginPlay`)

(event `self.ReceiveTick`
  (params (DeltaSeconds :type "Float (single-precision)"))
  (bind (_sun_rotation_roll _sun_rotation_pitch _sun_rotation_yaw) (`KismetMathLibrary.BreakRotator` (`self.Sun Rotation`)))
  (bind _returnvalue (* (`KismetSystemLibrary.GetGameTimeInSeconds`) (`self.Rotate Speed`)))
  (if (`self.Activate`)
    (if (`self.Rotate Cubemap`)
      ;[1 1 1] Update Rotation
      (`MaterialInstanceDynamic.SetScalarParameterValue` (`self.MI Skysphere`) "Rotation Angle" (+ (`self.Angle`) _returnvalue))
      (`SceneComponent.K2_SetWorldRotation` (`self.Directional Light angle`) (`KismetMathLibrary.MakeRotator` _sun_rotation_roll _sun_rotation_pitch (+ _sun_rotation_yaw (+ (`self.Angle`) _returnvalue))) false false)
      (`SkyLightComponent.RecaptureSky` (`self.SkyLight`)))))

(event `Switch Hyperspace Stage`
  (if (`self.4 Space`)
    ;[1 1 1] 1 Enter
    (set `self.4 Space` false)
    (set `self.1 Enter` true)
    (`|ExecutionSequence`
      (:`then_0`
        ;;[1 1 1] Dont use this Sky Light (Skylight in the BP_Hyperspace_Tunnel is turned on at this point)
        (`SceneComponent.SetVisibility` (`self.SkyLight`) false false))
      (:`then_1`
        ;;[1 1 1] Sky Sphere is not visible (Tunnel is turned on in BP_Hyoersoace_Tunnel)
        (`KismetSystemLibrary.Delay` 1.6)
        (`SceneComponent.SetVisibility` (`self.SkySphere_Reversed`) false false))
      (:`then_2`
        ;;[1 1 1] Sun is turned off
        (`KismetSystemLibrary.Delay` 1.6)
        (`SceneComponent.SetVisibility` (`self.DirectionalLight`) false false)
        (`SceneComponent.SetVisibility` (`self.Sun`) false false))
      (:`then_3`
        (`KismetSystemLibrary.Delay` 1.8)
        (set `self.1 Enter` false)
        ;[1 1 1] 2 Tunnel
        (set `self.2 Tunnel` true)))
    (elif (`self.2 Tunnel`)
      ;[1 1 1] 3 Exit
      (set `self.2 Tunnel` false)
      (set `self.3 Exit` true)
      (`|ExecutionSequence`
        (:`then_1`
          ;;[1 1 1] Space Sky Sphere is  visible
          (`KismetSystemLibrary.Delay` 1.4)
          (`SceneComponent.SetVisibility` (`self.SkySphere_Reversed`) true false))
        (:`then_3`
          ;;[1 1 1] Sun is turned on (Entering system of that sun)
          (`KismetSystemLibrary.Delay` 1.3)
          (`SceneComponent.SetVisibility` (`self.DirectionalLight`) true false)
          (`SceneComponent.SetVisibility` (`self.Sun`) true false))
        (:`then_4`
          (`KismetSystemLibrary.Delay` 1.56)
          (set `self.3 Exit` false)
          ;[1 1 1] 4 Space
          (set `self.4 Space` true)
          (`SceneComponent.SetVisibility` (`self.SkyLight`) true false)
          ;;[1 1 1] Recapture Skylight
          (`SkyLightComponent.RecaptureSky` (`self.SkyLight`)))))))

(fn `UserConstructionScript`
  (bind (_sun_rotation_roll _sun_rotation_pitch _sun_rotation_yaw) (`KismetMathLibrary.BreakRotator` (`self.Sun Rotation`)))
  (bind _sun (`self.Sun`))
  (if (`self.Activate`)
    (`SceneComponent.SetVisibility` (`self.SkySphere_Reversed`) true false)
    (`SceneComponent.SetVisibility` (`self.SkyLight`) true false)
    (`SceneComponent.SetVisibility` (`self.DirectionalLight`) true false)
    (`SceneComponent.SetVisibility` (`self.Sun`) true false)
    (`|ExecutionSequence`
      (:`then_0`
        ;[1 1 1] Material Parameters Skysphere
        (bind _returnvalue (`KismetMaterialLibrary.CreateDynamicMaterialInstance` "/Game/Maps/TestBeds/Mechanics/Studio_Lighting/M_SkySphere001.M_SkySphere001"))
        (bind _output_get (set `self.MI Skysphere` _returnvalue))
        (`PrimitiveComponent.SetMaterial` (`self.SkySphere_Reversed`) 0 _output_get)
        (`MaterialInstanceDynamic.SetScalarParameterValue` _output_get "Rotation Angle" (`self.Angle`))
        (`MaterialInstanceDynamic.SetTextureParameterValue` _output_get "HDRI Cubemap" (`self.Cubemap`))
        (`MaterialInstanceDynamic.SetTextureParameterValue` _output_get "PNG" (`self.PNG`))
        (`MaterialInstanceDynamic.SetVectorParameterValue` _output_get "Color Sky" (`self.Color Sky`))
        (`MaterialInstanceDynamic.SetVectorParameterValue` _output_get "Color Floor" (`self.Color Floor`))
        (`MaterialInstanceDynamic.SetScalarParameterValue` _output_get "Sky-Floor Blend" (`self.Sky-Floor Blend`))
        (`MaterialInstanceDynamic.SetVectorParameterValue` _output_get "Color Multiply" (`self.Color Multiply`))
        (`MaterialInstanceDynamic.SetScalarParameterValue` _output_get "Intensity" (`self.Intensity`))
        (`MaterialInstanceDynamic.SetScalarParameterValue` _output_get "Type Index" (`self.Type Index`)))
      (:`then_3`
        ;[1 1 1] Directional Light
        (`SceneComponent.K2_SetWorldRotation` (`self.Directional Light angle`) (`KismetMathLibrary.MakeRotator` _sun_rotation_roll _sun_rotation_pitch (+ _sun_rotation_yaw (`self.Angle`))) false false)
        (`LightComponent.SetLightColor` (`self.DirectionalLight`) (`self.Directional Light Color`) true)
        (`LightComponent.SetIntensity` (`self.DirectionalLight`) (`self.Directional Light Intensity`)))
      (:`then_4`
        ;[1 1 1] Sun
        (`SceneComponent.SetRelativeScale3D` (`self.Sun`) (`KismetMathLibrary.Conv_DoubleToVector` (`self.Sun Scale`)))
        ;;[1 1 1] Material Parameters Sun
        (bind _returnvalue_2 (`KismetMaterialLibrary.CreateDynamicMaterialInstance` "/Game/Maps/TestBeds/Mechanics/Studio_Lighting/M_Sun.M_Sun"))
        (bind _output_get_2 (set `self.MI Sun` _returnvalue_2))
        (`PrimitiveComponent.SetMaterial` (`self.Sun`) 0 _output_get_2)
        (`MaterialInstanceDynamic.SetVectorParameterValue` _output_get_2 "Color Sun" (`self.Color Sun`))
        (`MaterialInstanceDynamic.SetScalarParameterValue` _output_get_2 "Base Intensity" (`self.Sun Base Intensity`))
        (if (`self.Visualize Sun Position`)
          (`SceneComponent.SetVisibility` _sun true false)
          (else
            (`SceneComponent.SetVisibility` _sun false false))))
      (:`then_5`
        ;[1 1 1] Recapture Skylight
        (`SkyLightComponent.RecaptureSky` (`self.SkyLight`))))
    (else
      (`SceneComponent.SetVisibility` (`self.SkySphere_Reversed`) false false)
      (`SceneComponent.SetVisibility` (`self.SkyLight`) false false)
      (`SceneComponent.SetVisibility` (`self.DirectionalLight`) false false)
      (`SceneComponent.SetVisibility` (`self.Sun`) false false))))