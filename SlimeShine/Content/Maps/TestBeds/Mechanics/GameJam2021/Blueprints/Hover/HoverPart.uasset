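; A hovering platform piece that drops under a slime character carrying more active abilities than it supports.
; While the slime overlaps the box, overlap and Tick checks call EnableGrav, which switches on mesh physics and gravity.
; On exit physics switches off, and after a short delay a timeline lerps the mesh back to its start, stopping if a slime re-enters.
; A line-trace thrust calculation is left unconnected.
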(event `self.ReceiveBeginPlay`
  (set `self.StartLocation` (`SceneComponent.K2_GetComponentLocation` (`self.StaticMesh`))))

(event `self.Box.OnComponentBeginOverlap`
  (params (OverlappedComponent :type "PrimitiveComponent Object Reference") (OtherActor :type "Actor Object Reference") (OtherComp :type "PrimitiveComponent Object Reference") (OtherBodyIndex :type Integer) (bFromSweep :type Boolean) (SweepResult :type "HitResult Structure (by ref)"))
  (`self.EnableGrav` OtherActor))

(event `self.Box.OnComponentEndOverlap`
  (params (OverlappedComponent :type "PrimitiveComponent Object Reference") (OtherActor :type "Actor Object Reference") (OtherComp :type "PrimitiveComponent Object Reference") (OtherBodyIndex :type Integer))
  (bind _staticmesh (`self.StaticMesh`))
  (bind _returnvalue (== (`KismetArrayLibrary.Array_Length` (`PrimitiveComponent.GetOverlappingActors` (`self.Box`) "/Game/Maps/TestBeds/Mechanics/GameJam2021/BP_Slime_Character.BP_Slime_Character_C")) 0))
  (cast `/Game/Maps/TestBeds/Mechanics/GameJam2021/BP_Slime_Character` OtherActor)
  (`PrimitiveComponent.SetSimulatePhysics` _staticmesh false)
  (`PrimitiveComponent.SetEnableGravity` _staticmesh false)
  (`KismetSystemLibrary.Delay` 0.7)
  (if _returnvalue
    (set `self.RelocateLocation` (`SceneComponent.K2_GetComponentLocation` (`self.StaticMesh`)))
    (bind (_direction _time) (`Timeline|BackToPos` :!via `PlayFromStart` :!label _label)
      (:`Update`
        (`SceneComponent.K2_SetWorldLocation` (`self.StaticMesh`) (`KismetMathLibrary.VLerp` (`self.RelocateLocation`) (`self.StartLocation`) _time) false false)
        (if (not _returnvalue)
          (`|ExecutionSequence`
            (:`then_0`
              (goto _label :!via `Stop`))
            (:`then_1`
              (`self.EnableGrav` (`GameplayStatics.GetPlayerPawn` 0)))))))))

(event `self.ReceiveTick`
  (params (DeltaSeconds :type "Float (single-precision)"))
  (if (not (== (`KismetArrayLibrary.Array_Length` (`PrimitiveComponent.GetOverlappingActors` (`self.Box`) "/Game/Maps/TestBeds/Mechanics/GameJam2021/BP_Slime_Character.BP_Slime_Character_C")) 0))
    (`self.EnableGrav` (`GameplayStatics.GetPlayerPawn` 0))))

(fn `EnableGrav`
  (params (Object :type "Object Object Reference"))
  (bind _staticmesh (`self.StaticMesh`))
  (bind _asbp_slime_character (cast `/Game/Maps/TestBeds/Mechanics/GameJam2021/BP_Slime_Character` Object))
  (bind _count (`/Game/Maps/TestBeds/Mechanics/GameJam2021/BP_Slime_Character.ActiveAbilitiesCount` _asbp_slime_character))
  (if (> _count (`self.MaxSupportedAbilities`))
    (`PrimitiveComponent.SetSimulatePhysics` _staticmesh true)
    (`PrimitiveComponent.SetEnableGravity` _staticmesh true)))

(fn `UserConstructionScript`)