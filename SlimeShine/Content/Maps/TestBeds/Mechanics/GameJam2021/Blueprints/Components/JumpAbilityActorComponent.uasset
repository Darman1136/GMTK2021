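; Jump ability component for a GameJam 2021 test bed that launches the owning character's physics actor along its gravity axis.
; Each tick it sets Ready from a cooldown since the last jump, using a Delay while falling as a coyote-time grace window before disabling the jump.
; Using the ability records the jump time and applies an impulse of GravityDirection scaled by Impulse.Z, supporting arbitrary gravity directions.
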(event `self.ReceiveTick`
  (params (DeltaSeconds :type "Float (single-precision)"))
  (`parent.ReceiveTick` DeltaSeconds)
  (`|ExecutionSequence`
    (:`then_0`
      (if (`/Game/Maps/TestBeds/Mechanics/GameJam2021/BP_Slime_Character.IsFalling` (`self.CastedCharacter`))
        (`KismetSystemLibrary.Delay` (`self.JumpAllowanceS`))
        (if (`/Game/Maps/TestBeds/Mechanics/GameJam2021/BP_Slime_Character.IsFalling` (`self.CastedCharacter`))
          (set `self.Ready` false)
          (else
            (if (> (- (`KismetMathLibrary.GetTotalMilliseconds` (`KismetMathLibrary.FromSeconds` (`GameplayStatics.GetRealTimeSeconds`))) (`self.LastJump`)) (`self.JumpDelayMs`)) :!label _label
              (set `self.Ready` true)
              (else
                (set `self.Ready` false)))))
        (else
          (goto _label))))))

(fn `InternalUseAbility`
  (returns (Success :type Boolean))
  (bind _castedcharacter (`self.CastedCharacter`))
  (bind (_impulse_x _impulse_y _impulse_z) (`KismetMathLibrary.BreakVector` (`self.Impulse`)))
  (set `self.LastJump` (`KismetMathLibrary.GetTotalMilliseconds` (`KismetMathLibrary.FromSeconds` (`GameplayStatics.GetRealTimeSeconds`))))
  (`PrimitiveComponent.AddImpulse` (`/Game/Maps/TestBeds/Mechanics/GameJam2021/BP_Slime_Character.GetPhysicsActor` _castedcharacter) (* (`/Game/Maps/TestBeds/Mechanics/GameJam2021/BP_Slime_Character.GravityDirection` _castedcharacter) _impulse_z) "None" false)
  (return true))