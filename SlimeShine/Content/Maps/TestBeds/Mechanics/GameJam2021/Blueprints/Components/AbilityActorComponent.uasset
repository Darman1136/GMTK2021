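; AbilityActorComponent is a base component for slime character abilities in a 2021 game jam test bed.
; On BeginPlay it caches its owner as a BP_Slime_Character.
; UseAbility runs the overridable InternalUseAbility only when the ability is enabled, ready and not temporarily disabled, returning its result.
; Enable sets the flag, calls the overridable InternalEnable hook and broadcasts the EnableEd dispatcher.
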(event `self.ReceiveBeginPlay`
  (bind _asbp_slime_character (cast `/Game/Maps/TestBeds/Mechanics/GameJam2021/BP_Slime_Character` (`self.GetOwner`)))
  (set `self.CastedCharacter` _asbp_slime_character))

(fn `Enable`
  (params (Enable :type Boolean))
  (bind _output_get (set `self.Enabled` Enable))
  (`self.InternalEnable` _output_get)
  (`self.EnableEd` _output_get self))

(fn `InternalEnable`
  (params (Enable :type Boolean)))

(fn `InternalUseAbility`
  (returns (Success :type Boolean))
  (return false))

(fn `IsEnabled`
  (returns (Enabled :type Boolean))
  (return (`self.Enabled`)))

(fn `IsReady`
  (returns (Ready :type Boolean))
  (return (and (`self.IsEnabled`) (`self.Ready`) (not (`self.TemporarilyDisabled`)))))

(fn `UseAbility`
  (returns (Success :type Boolean))
  (if (`self.IsReady`)
    (bind _success (`self.InternalUseAbility`))
    (return _success)
    (else
      (return false))))