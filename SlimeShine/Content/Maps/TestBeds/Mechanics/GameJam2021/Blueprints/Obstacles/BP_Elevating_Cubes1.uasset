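; BP_Elevating_Cubes1 is a game jam obstacle: a cube that continuously bobs up and down.
; BeginPlay stores the Cube component's world location as the origin.
; Each Tick sets the cube's height to that origin plus a sine of game time, scaled by speed and height multipliers, leaving X and Y fixed.
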(event `self.ReceiveBeginPlay`
  ;[1 1 1] Set initial Location
  (set `self.Initial Location Right` (`SceneComponent.K2_GetComponentLocation` (`self.Cube`))))

(event `self.ReceiveTick`
  (params (DeltaSeconds :type "Float (single-precision)"))
  (bind (_initial_location_right_x _initial_location_right_y _initial_location_right_z) (`KismetMathLibrary.BreakVector` (`self.Initial Location Right`)))
  (`SceneComponent.K2_SetWorldLocation` (`self.Cube`) (`KismetMathLibrary.MakeVector` _initial_location_right_x _initial_location_right_y (+ _initial_location_right_z (* (`KismetMathLibrary.Sin` (* (`KismetSystemLibrary.GetGameTimeInSeconds`) (`self.Speed Multiplier`))) (`self.Height Multiplier`)))) false false))

(fn `UserConstructionScript`)