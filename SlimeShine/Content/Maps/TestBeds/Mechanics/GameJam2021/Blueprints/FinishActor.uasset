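; FinishActor is a level goal that loads the next level when the slime character touches it.
; On begin play it hides its mesh, attaches a Niagara finish effect to a slowly rotating sphere and fades in background music.
; Overlap by BP_Slime_Character marks it finished, plays sound cues, fades the music out and opens LevelName after a delay.
; Meanwhile a timeline drives the effect's scale curve and an absorb effect spawns.
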(event `self.ReceiveBeginPlay`
  (`|ExecutionSequence`
    (:`then_0`
      (`SceneComponent.SetVisibility` (`self.StaticMesh`) false false)
      (bind _returnvalue (`NiagaraFunctionLibrary.SpawnSystemAttached` "/Game/Maps/TestBeds/Mechanics/GameJam2021/Niagara/NS_Slime_Finish.NS_Slime_Finish" (`self.Sphere`) "None" (0.0 0.0 0.0) (struct) "KeepRelativeOffset"))
      (set `self.Niagara System Pickup` _returnvalue))
    (:`then_1`
      (`TimelineComponent.SetPlayRate` (`self.Hovering`) (/ 1.0 10.0))
      (bind (_direction _newtrack_0) (`Timeline|Hovering` :!via `PlayFromStart`)
        (:`Update`
          (bind _returnvalue_2 (* _newtrack_0 360.0))
          (`SceneComponent.K2_SetWorldRotation` (`self.Sphere`) (`KismetMathLibrary.MakeRotator` 0.0 _returnvalue_2 _returnvalue_2) false false))))
    (:`then_3`
      (`AudioComponent.FadeIn` (`self.BgMusic_Cue`) 0.0 1.0 0.0 "Linear"))))

(event `self.Sphere.OnComponentBeginOverlap`
  (params (OverlappedComponent :type "PrimitiveComponent Object Reference") (OtherActor :type "Actor Object Reference") (OtherComp :type "PrimitiveComponent Object Reference") (OtherBodyIndex :type Integer) (bFromSweep :type Boolean) (SweepResult :type "HitResult Structure (by ref)"))
  (cast `/Game/Maps/TestBeds/Mechanics/GameJam2021/BP_Slime_Character` OtherActor)
  (`self.Finish`)
  (`|ExecutionSequence`
    (:`then_0`
      (bind (_direction _newtrack_0) (`Timeline|Timeline_0` :!via `PlayFromStart`)
        (:`Update`
          (`FXSystemComponent.SetFloatParameter` (`self.Niagara System Pickup`) "Scale Curve" _newtrack_0))))
    (:`then_1`
      (`NiagaraFunctionLibrary.SpawnSystemAttached` "/Game/Maps/TestBeds/Mechanics/Droideka/Special_Effects/Collision_Sparks/NE_Slime_Finish_Absorb.NE_Slime_Finish_Absorb" (`self.Sphere`) "None" (0.0 0.0 0.0) (struct) "KeepRelativeOffset"))))

(event `Finish`
  (set `self.Finished` true)
  (`AudioComponent.Play` (`self.Cue_On_Cut`) 0.0)
  (`AudioComponent.Play` (`self.Cue_On_Join1`) 0.0)
  (`AudioComponent.FadeOut` (`self.BgMusic_Cue`) 2.0 0.0 "Linear")
  (`KismetSystemLibrary.Delay` 2.0)
  (`GameplayStatics.OpenLevel` (`self.Level Name`)))

(fn `UserConstructionScript`)