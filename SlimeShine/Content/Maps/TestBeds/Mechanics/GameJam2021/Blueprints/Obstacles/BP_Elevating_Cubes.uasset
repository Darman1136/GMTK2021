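; BP_Elevating_Cubes is a game jam obstacle with two cubes that continuously bob up and down.
; BeginPlay caches each cube's world location, and Tick offsets its Z by a sine of game time scaled by HeightMultiplier.
; The left cube's sine runs at a higher frequency than the right's, so the two drift in and out of sync.
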(event `self.ReceiveBeginPlay`
  ;[1 1 1] Set initial Location
  (set `self.Initial Location Right` (`SceneComponent.K2_GetComponentLocation` (`self.Cube Right`)))
  (set `self.Initial Location Left` (`SceneComponent.K2_GetComponentLocation` (`self.Cube Left`))))

(event `self.ReceiveTick`
  (params (DeltaSeconds :type "Float (single-precision)"))
  (bind (_initial_location_right_x _initial_location_right_y _initial_location_right_z) (`KismetMathLibrary.BreakVector` (`self.Initial Location Right`)))
  (bind (_initial_location_left_x _initial_location_left_y _initial_location_left_z) (`KismetMathLibrary.BreakVector` (`self.Initial Location Left`)))
  (`SceneComponent.K2_SetWorldLocation` (`self.Cube Right`) (`KismetMathLibrary.MakeVector` _initial_location_right_x _initial_location_right_y (+ _initial_location_right_z (* (`KismetMathLibrary.Sin` (`KismetSystemLibrary.GetGameTimeInSeconds`)) (`self.Height Multiplier`)))) false false)
  (`SceneComponent.K2_SetWorldLocation` (`self.Cube Left`) (`KismetMathLibrary.MakeVector` _initial_location_left_x _initial_location_left_y (+ _initial_location_left_z (* (`KismetMathLibrary.Sin` (* (`KismetSystemLibrary.GetGameTimeInSeconds`) 1.333)) (`self.Height Multiplier`)))) false false))

(fn `UserConstructionScript`)