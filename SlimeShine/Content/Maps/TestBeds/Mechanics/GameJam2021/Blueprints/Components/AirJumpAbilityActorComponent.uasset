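; Actor component from a game jam test bed that grants the character a single air jump after it leaves the ground.
; Tick compares the previous grounded state with the current falling state to set Ready, clearing it once the jump is used or the character lands.
; Using the ability flags Jumped and adds an impulse to the physics actor along the gravity direction, scaled by Impulse Z, so it follows the character's own gravity.
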(event `self.ReceiveTick`
  (params (DeltaSeconds :type "Float (single-precision)"))
  (bind _falling (`/Game/Maps/TestBeds/Mechanics/GameJam2021/BP_Slime_Character.IsFalling` (`self.CastedCharacter`)))
  (bind _returnvalue (not _falling))
  (`parent.ReceiveTick` DeltaSeconds)
  (`|ExecutionSequence`
    (:`then_0`
      (if (and (`self.WasOnGround`) _falling (not (`self.Jumped`)))
        (set `self.Ready` true)))
    (:`then_1`
      (if (and _falling (`self.Jumped`))
        (set `self.Ready` false)))
    (:`then_2`
      (if (and _returnvalue (`self.Jumped`))
        (set `self.Jumped` false)))
    (:`then_3`
      (if (and (`self.Ready`) _returnvalue)
        (set `self.Ready` false)))
    (:`then_4`
      (set `self.WasOnGround` _returnvalue))))

(fn `InternalUseAbility`
  (returns (Success :type Boolean))
  (bind _castedcharacter (`self.CastedCharacter`))
  (bind (_impulse_x _impulse_y _impulse_z) (`KismetMathLibrary.BreakVector` (`self.Impulse`)))
  (set `self.Jumped` true)
  (`PrimitiveComponent.AddImpulse` (`/Game/Maps/TestBeds/Mechanics/GameJam2021/BP_Slime_Character.GetPhysicsActor` _castedcharacter) (* (`/Game/Maps/TestBeds/Mechanics/GameJam2021/BP_Slime_Character.GravityDirection` _castedcharacter) _impulse_z) "None" false)
  (return true))