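; Moving cube obstacle from a GameJam 2021 test bed that slides back and forth along world X.
; BeginPlay caches the cube component's world location as the centre of the motion.
; Each Tick offsets X by the sine of game time scaled by LocationMultiplier, keeping Y and Z fixed.
; Motion follows absolute game time rather than accumulated deltas, so all instances share the same phase.
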(event `self.ReceiveBeginPlay`
  (set `self.Initial Location` (`SceneComponent.K2_GetComponentLocation` (`self.Cube`))))

(event `self.ReceiveTick`
  (params (DeltaSeconds :type "Float (single-precision)"))
  (bind (_initial_location_x _initial_location_y _initial_location_z) (`KismetMathLibrary.BreakVector` (`self.Initial Location`)))
  (`SceneComponent.K2_SetWorldLocation` (`self.Cube`) (`KismetMathLibrary.MakeVector` (+ _initial_location_x (* (`KismetMathLibrary.Sin` (`KismetSystemLibrary.GetGameTimeInSeconds`)) (`self.Location Multiplier`))) _initial_location_y _initial_location_z) false false))

(fn `UserConstructionScript`)