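; Game jam slime Blueprint that rebuilds its Niagara sphere effects each time OnJoin is called.
; Each call spawns one attached NS_Slime_Sphere per entry in Colors, tinted to that color, splitting a fixed particle budget by NumColors.
; A FlipFlop alternates two component arrays as a double buffer, so the new systems appear while a timeline rescales the old ones, then destroys them.
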(event `On Join`
  (bind _niagara_systems_a (`self.Niagara Systems A`))
  (bind _niagara_systems_b (`self.Niagara Systems B`))
  ;[1 1 1] Destory Old, Spawn New (Which will be old the next time)
  (`/Engine/EditorBlueprintResources/StandardMacros.FlipFlop`
    (:`A`
      (`|ExecutionSequence`
        (:`then_0`
          ;[1 1 1] Destory old Systems
          (bind (_direction _scale_lerp) (`Timeline|Timeline_0` :!via `PlayFromStart`)
            (:`Update`
              (for _array_element (`self.Niagara Systems A`)
                (`SceneComponent.SetWorldScale3D` _array_element (* (1.0 1.0 1.0) _scale_lerp))))
            (:`Finished`
              (for _array_element_2 _niagara_systems_a
                (`ActorComponent.K2_DestroyComponent` _array_element_2))
              (`KismetArrayLibrary.Array_Clear` _niagara_systems_a))))
        (:`then_1`
          ;[1 1 1] Spawn New Systems
          (for _array_element_3 (`self.Colors`)
            (bind _returnvalue (`NiagaraFunctionLibrary.SpawnSystemAttached` "/Game/Maps/TestBeds/Mechanics/GameJam2021/Niagara/NS_Slime_Sphere.NS_Slime_Sphere" null "None" (0.0 0.0 0.0) (struct) "SnapToTarget"))
            (`FXSystemComponent.SetColorParameter` _returnvalue "Color" _array_element_3)
            (`NiagaraComponent.SetVariableInt` _returnvalue "Spawn Count" (/ 1000 (`self.NumColors`)))
            (`KismetArrayLibrary.Array_Add` (`self.Niagara Systems B`) _returnvalue)))))
    (:`B`
      (`|ExecutionSequence`
        (:`then_0`
          ;[1 1 1] Destory old Systems
          (bind (_direction_2 _scale_lerp_2) (`Timeline|Timeline_1` :!via `PlayFromStart`)
            (:`Update`
              (for _array_element_4 (`self.Niagara Systems B`)
                (`SceneComponent.SetWorldScale3D` _array_element_4 (* (1.0 1.0 1.0) _scale_lerp_2))))
            (:`Finished`
              (for _array_element_5 _niagara_systems_b
                (`ActorComponent.K2_DestroyComponent` _array_element_5))
              (`KismetArrayLibrary.Array_Clear` _niagara_systems_b))))
        (:`then_1`
          ;[1 1 1] Spawn New Systems
          (for _array_element_6 (`self.Colors`)
            (bind _returnvalue_2 (`NiagaraFunctionLibrary.SpawnSystemAttached` "/Game/Maps/TestBeds/Mechanics/GameJam2021/Niagara/NS_Slime_Sphere.NS_Slime_Sphere" null "None" (0.0 0.0 0.0) (struct) "SnapToTarget"))
            (`FXSystemComponent.SetColorParameter` _returnvalue_2 "Color" _array_element_6)
            (`NiagaraComponent.SetVariableInt` _returnvalue_2 "Spawn Count" (/ 1000 (`self.NumColors`)))
            (`KismetArrayLibrary.Array_Add` (`self.Niagara Systems A`) _returnvalue_2)))))))

(fn `UserConstructionScript`)