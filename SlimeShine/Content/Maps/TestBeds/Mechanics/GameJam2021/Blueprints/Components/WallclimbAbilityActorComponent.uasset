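; Wall-climb ability component from a 2021 game jam test bed that reorients the owning character's gravity to surfaces it hits.
; While enabled, it binds to hit events on the character's physics actor.
; Hits on static mesh actors print the impact normal and, unless the surface faces noticeably downward, assign that normal as the gravity direction.
; Tick marks the ability ready whenever the character is not falling.
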(event `self.ReceiveBeginPlay`
  (`parent.ReceiveBeginPlay`))

(event `self.ReceiveTick`
  (params (DeltaSeconds :type "Float (single-precision)"))
  (`parent.ReceiveTick` DeltaSeconds)
  (set `self.Ready` (not (`/Game/Maps/TestBeds/Mechanics/GameJam2021/BP_Slime_Character.IsFalling` (`self.CastedCharacter`)))))

(event `PhyActorHit`
  (params (HitComponent :type "PrimitiveComponent Object Reference") (OtherActor :type "Actor Object Reference") (OtherComp :type "PrimitiveComponent Object Reference") (NormalImpulse :type "Vector Structure") (Hit :type "HitResult Structure (by ref)"))
  (bind (_bblockinghit _binitialoverlap _time _distance _location _impactpoint _normal _impactnormal) (`GameplayStatics.BreakHitResult` Hit))
  (cast `StaticMeshActor` OtherActor)
  (`KismetSystemLibrary.PrintString` (`KismetStringLibrary.Conv_VectorToString` _impactnormal))
  (if (> (.z _impactnormal) -0.1)
    (set `/Game/Maps/TestBeds/Mechanics/GameJam2021/BP_Slime_Character.GravityDirection` _impactnormal (`self.CastedCharacter`))))

(fn `InternalEnable`
  (params (Enable :type Boolean))
  (`parent.InternalEnable` Enable)
  (if Enable
    (add `PrimitiveComponent.OnComponentHit` (`/Game/Maps/TestBeds/Mechanics/GameJam2021/BP_Slime_Character.GetPhysicsActor` (`self.CastedCharacter`)) (`|CreateDelegate` :!event `PhyActorHit`))
    (else
      (remove `PrimitiveComponent.OnComponentHit` (`/Game/Maps/TestBeds/Mechanics/GameJam2021/BP_Slime_Character.GetPhysicsActor` (`self.CastedCharacter`)) (`|CreateDelegate` :!event `PhyActorHit`)))))