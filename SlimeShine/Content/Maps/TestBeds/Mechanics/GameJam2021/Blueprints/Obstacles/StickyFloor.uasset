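; Sticky floor obstacle that disables the slime character's dash ability while the slime stands within it.
; Overlap begin on the static mesh sets the dash component's temporary disable flag and shows a "Dash unavailable" message on the in-game HUD.
; Overlap end clears the flag and hides the message, with no counting of overlapping floors.
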(event `self.StaticMesh.OnComponentBeginOverlap`
  (params (OverlappedComponent :type "PrimitiveComponent Object Reference") (OtherActor :type "Actor Object Reference") (OtherComp :type "PrimitiveComponent Object Reference") (OtherBodyIndex :type Integer) (bFromSweep :type Boolean) (SweepResult :type "HitResult Structure (by ref)"))
  (bind _asbp_slime_character (cast `/Game/Maps/TestBeds/Mechanics/GameJam2021/BP_Slime_Character` OtherActor))
  (set `/Game/Maps/TestBeds/Mechanics/GameJam2021/Blueprints/Components/AbilityActorComponent.TemporarilyDisabled` true (`/Game/Maps/TestBeds/Mechanics/GameJam2021/BP_Slime_Character.DashAbilityActorComponent` _asbp_slime_character))
  (`/Game/Maps/TestBeds/Mechanics/GameJam2021/Blueprints/HUD/Ingame.ShowDisabled` (`/Game/Maps/TestBeds/Mechanics/GameJam2021/BP_Slime_Character.IngameHud` _asbp_slime_character) "Dash unavailable"))

(event `self.StaticMesh.OnComponentEndOverlap`
  (params (OverlappedComponent :type "PrimitiveComponent Object Reference") (OtherActor :type "Actor Object Reference") (OtherComp :type "PrimitiveComponent Object Reference") (OtherBodyIndex :type Integer))
  (bind _asbp_slime_character (cast `/Game/Maps/TestBeds/Mechanics/GameJam2021/BP_Slime_Character` OtherActor))
  (set `/Game/Maps/TestBeds/Mechanics/GameJam2021/Blueprints/Components/AbilityActorComponent.TemporarilyDisabled` false (`/Game/Maps/TestBeds/Mechanics/GameJam2021/BP_Slime_Character.DashAbilityActorComponent` _asbp_slime_character))
  (`/Game/Maps/TestBeds/Mechanics/GameJam2021/Blueprints/HUD/Ingame.HideDisabled` (`/Game/Maps/TestBeds/Mechanics/GameJam2021/BP_Slime_Character.IngameHud` _asbp_slime_character)))

(fn `UserConstructionScript`)